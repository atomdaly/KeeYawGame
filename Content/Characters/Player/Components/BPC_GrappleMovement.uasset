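; Player component for a swinging grapple hook, fired along the camera view at any Visibility trace hit.
; A looping 0.1s timer capsule-traces to update the crosshair and, while a gate is open, moves the rope toward the hook and applies velocity-based pendulum force.
; Grappling launches the player upward and alters gravity and air control; reset or grapple jump restores them.
; The "Grapple" tag filters, pull-in launch and cancel-condition expression are disconnected.
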(event `InitializeGrapple`
  (params (Character :type "/Game/Characters/Player/BP_PlayerCharacter Object Reference") (GrappleRope :type "CableComponent Object Reference"))
  (bind _output_get (set `self.Player` Character))
  (bind _output_get_2 (set `self.CharacterMovement` (`Character.CharacterMovement` _output_get)))
  (set `self.DefaultGravity` (`CharacterMovementComponent.GravityScale` _output_get_2))
  (set `self.DefaultAirControl` (`CharacterMovementComponent.AirControl` _output_get_2))
  (set `self.GrappleRope` GrappleRope)
  (bind _returnvalue (`GameplayStatics.GetActorOfClass` "/Game/Core/Blueprints/BP_LevelManager.BP_LevelManager_C"))
  (set `self.HUD` (`/Game/Core/Blueprints/BP_LevelManager.HUD` _returnvalue))
  (`KismetSystemLibrary.K2_SetTimerDelegate` (delegate `ShootGrapple`) 0.1 true))

(event `ShootGrapple`
  (bind _player (`self.Player`))
  (bind _grapplerope (`self.GrappleRope`))
  (bind _crosshair (`/Game/UI/WBP_HUD.Crosshair` (`self.HUD`)))
  (bind _playercamera (`/Game/Characters/Player/BP_PlayerCharacter.PlayerCamera` (`self.Player`)))
  (bind _returnvalue (- (`Actor.K2_GetActorLocation` _player) (`self.HookLocation`)))
  (bind _returnvalue_2 (`SceneComponent.K2_GetComponentLocation` _playercamera))
  (bind (_outhit _returnvalue_3) (`KismetSystemLibrary.CapsuleTraceSingle` _returnvalue_2 (+ _returnvalue_2 (* (`SceneComponent.GetForwardVector` _playercamera) 5000.0)) 75.0 0.0 "TraceTypeQuery1"))
  (if _returnvalue_3
    (`Image.SetBrush` _crosshair (`self.GrappleCrosshair`))
    (else
      (`Image.SetBrush` _crosshair (`self.DefaultCrosshair`))))
  (`/Engine/EditorBlueprintResources/StandardMacros.Gate` true :!label _label
    (:`Exit`
      (if (`self.GrappleCancelConditions`)
        (`self.ResetGrapple`)
        (else
          (`SceneComponent.SetVisibility` _grapplerope true false)
          (`SceneComponent.K2_SetWorldLocation` _grapplerope (`KismetMathLibrary.VInterpTo` (`SceneComponent.K2_GetComponentLocation` _grapplerope) (`self.HookLocation`) (`GameplayStatics.GetWorldDeltaSeconds`) 40.0) true false)
          (`CharacterMovementComponent.AddForce` (`self.CharacterMovement`) (* (* (`KismetMathLibrary.Normal` _returnvalue) (`KismetMathLibrary.Dot_VectorVector` (`Actor.GetVelocity` _player) _returnvalue)) -2.0)))))))

(event `OpenGrappleGate`
  (goto _label :!via `Open`))

(event `CloseGrappleGate`
  (goto _label :!via `Close`))

(event `GrappleEvent`
  (bind _charactermovement (`self.CharacterMovement`))
  (bind _playercamera (`/Game/Characters/Player/BP_PlayerCharacter.PlayerCamera` (`self.Player`)))
  (bind _returnvalue (`SceneComponent.K2_GetComponentLocation` _playercamera))
  (if (`self.bCanGrapple?`)
    (set `self.bCanGrapple?` false)
    (bind (_outhit _returnvalue_2) (`KismetSystemLibrary.CapsuleTraceSingle` _returnvalue (+ _returnvalue (* (`SceneComponent.GetForwardVector` _playercamera) 5000.0)) 75.0 0.0 "TraceTypeQuery1"))
    (if _returnvalue_2
      (set `self.OutHit` _outhit)
      (set `self.HookLocation` (`.Location` (`GameplayStatics.BreakHitResult` _outhit)))
      (`self.OpenGrappleGate`)
      (`Character.LaunchCharacter` (`self.Player`) (0.0 0.0 250.0) false false)
      (set `CharacterMovementComponent.AirControl` (`self.GrappleAirControl`) _charactermovement)
      (set `CharacterMovementComponent.GravityScale` 0.5 _charactermovement)
      (else
        (`self.ResetGrapple`)))
    (else
      (`self.ResetGrapple`))))

(event `ResetGrapple`
  (bind _charactermovement (`self.CharacterMovement`))
  (`SceneComponent.SetVisibility` (`self.GrappleRope`) false false)
  (`self.CloseGrappleGate`)
  (set `CharacterMovementComponent.GravityScale` (`self.DefaultGravity`) _charactermovement)
  (set `CharacterMovementComponent.AirControl` (`self.DefaultAirControl`) _charactermovement)
  (`KismetSystemLibrary.Delay` 0.2)
  (set `self.bCanGrapple?` true))

(event `GrappleJump`
  (if (not (`self.bCanGrapple?`))
    (`Character.LaunchCharacter` (`self.Player`) (0.0 0.0 750.0) false false)
    (`self.ResetGrapple`)))