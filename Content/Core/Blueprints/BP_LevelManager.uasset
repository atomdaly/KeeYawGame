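; Level manager actor that handles player spawning, course resets, the run timer and pausing.
; BeginPlay places the player at CheckPoint or BP_LevelStart, creates the HUD and starts a one-second timer gated by CanTick.
; Box overlap or ResetCourse returns the player to spawn and clears and hides the timer.
; Pausing possesses a BP_PauseMenuPawn aligned to the player camera; number keys provide level-load and slow-motion shortcuts.
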(event `self.ReceiveBeginPlay`
  (bind _playerspawntransform (`self.PlayerSpawnTransform`))
  (bind _checkpoint (`self.CheckPoint`))
  (bind (_returnvalue_location _returnvalue_rotation) (`KismetMathLibrary.BreakTransform` (`self.GetTransform` _checkpoint)))
  (bind _asbp_player_character (cast `/Game/Characters/Player/BP_PlayerCharacter` (`GameplayStatics.GetPlayerCharacter` 0)))
  (set `self.Player` _asbp_player_character)
  (bind _returnvalue (`GameplayStatics.GetActorOfClass` "/Game/Core/Blueprints/BP_LevelStart.BP_LevelStart_C"))
  (`/Engine/EditorBlueprintResources/StandardMacros.IsValid` _checkpoint
    (:`Is Valid`
      (set `self.PlayerSpawnTransform` (`KismetMathLibrary.MakeTransform` _returnvalue_location _returnvalue_rotation)))
    (:`Is Not Valid`
      (bind _returnvalue_2 (`self.GetTransform` _returnvalue))
      (set `self.PlayerSpawnTransform` (`KismetMathLibrary.MakeTransform` (`KismetMathLibrary.MakeVector` (.x (.location _returnvalue_2)) (.y (.location _returnvalue_2)) (+ (.z (.location _returnvalue_2)) 100.0)) (.rotation _returnvalue_2)))))
  (`self.K2_SetActorTransform` (`self.Player`) _playerspawntransform false true)
  (`Controller.SetControlRotation` (`GameplayStatics.GetPlayerController` 0) (`KismetMathLibrary.MakeRotator` 0.0 0.0 (.yaw (.rotation _playerspawntransform))))
  (`self.EnableInput` (`GameplayStatics.GetPlayerController` 0))
  (bind _returnvalue_3 (`GameplayStatics.GetActorOfClass` "/Game/UI/Blueprints/PauseMenu/BP_PauseMenuPawn.BP_PauseMenuPawn_C"))
  (set `self.PauseMenuPawn` _returnvalue_3)
  (`KismetSystemLibrary.K2_SetTimerDelegate` (delegate `LevelTimer`) 1.0 true)
  (bind _returnvalue_4 (`|CreateWidget` "/Game/UI/WBP_HUD.WBP_HUD_C"))
  (bind _output_get (set `self.HUD` _returnvalue_4))
  (`UserWidget.AddToViewport` _output_get 0)
  (`WidgetBlueprintLibrary.SetInputMode_GameOnly` (`GameplayStatics.GetPlayerController` 0)))

(event `LevelTimer`
  (bind _seconds (`self.Seconds`))
  (if (`self.bCanTick?`)
    (if (== _seconds 59)
      (set `self.Seconds` 0)
      (set `self.Minutes` (+ (`self.Minutes`) 1))
      (else
        (set `self.Seconds` (+ _seconds 1))))))

(event `SetLevel`
  (bind _playerspawntransform (`self.PlayerSpawnTransform`))
  (set `self.bCanTick?` false)
  (`self.K2_SetActorTransform` (`self.Player`) _playerspawntransform false true)
  (`Controller.SetControlRotation` (`GameplayStatics.GetPlayerController` 0) (`KismetMathLibrary.MakeRotator` 0.0 0.0 (.yaw (.rotation _playerspawntransform))))
  (`/Game/Characters/Player/BP_PlayerCharacter.ResetSprint` (`self.Player`))
  (set `self.Minutes` 0)
  (set `self.Seconds` 0)
  (bind _foundwidgets (`WidgetBlueprintLibrary.GetAllWidgetsOfClass` "/Game/UI/WBP_Timer.WBP_Timer_C" false))
  (`Widget.SetVisibility` (`|GetArrayItem` _foundwidgets) "Hidden"))

(event `self.Box.OnComponentBeginOverlap`
  (params (OverlappedComponent :type "PrimitiveComponent Object Reference") (OtherActor :type "Actor Object Reference") (OtherComp :type "PrimitiveComponent Object Reference") (OtherBodyIndex :type Integer) (bFromSweep :type Boolean) (SweepResult :type "HitResult Structure (by ref)"))
  (if (== OtherActor (`GameplayStatics.GetPlayerCharacter` 0))
    (`self.SetLevel`)))

(event `OpenMenu`
  (bind _pausemenupawn (`self.PauseMenuPawn`))
  (bind _pausemenupawn_2 (`self.PauseMenuPawn`))
  (bind _player (`self.Player`))
  (set `self.bMenuOpen` true)
  (`self.FindMenuPawn`)
  (`SceneComponent.K2_SetWorldLocationAndRotation` (`Actor.RootComponent` _pausemenupawn) (`self.K2_GetActorLocation` _player) (`self.K2_GetActorRotation` _player) false false)
  (`SceneComponent.K2_SetWorldRotation` (`/Game/UI/Blueprints/PauseMenu/BP_PauseMenuPawn.Camera` _pausemenupawn) (`SceneComponent.K2_GetComponentRotation` (`/Game/Characters/Player/BP_PlayerCharacter.PlayerCamera` _player)) false false)
  (set `/Game/UI/Blueprints/PauseMenu/BP_PauseMenuPawn.GamepadInput` (`self.GamepadInput`) _pausemenupawn_2)
  (`Controller.Possess` (`GameplayStatics.GetPlayerController` 0) _pausemenupawn_2)
  (`GameplayStatics.SetGamePaused` true)
  (`Widget.SetVisibility` (`self.HUD`) "Hidden"))

(event `CloseMenu`
  (bind _returnvalue (`GameplayStatics.GetPlayerController` 0))
  (`GameplayStatics.SetGamePaused` false)
  (`Controller.SetControlRotation` _returnvalue (`SceneComponent.K2_GetComponentRotation` (`/Game/UI/Blueprints/PauseMenu/BP_PauseMenuPawn.Camera` (`self.PauseMenuPawn`))))
  (`Controller.Possess` _returnvalue (`self.Player`))
  (`self.EnableInput` (`GameplayStatics.GetPlayerController` 0))
  (set `self.bMenuOpen` false)
  (`Widget.SetVisibility` (`self.HUD`) "Visible")
  (bind _foundwidgets (`WidgetBlueprintLibrary.GetAllWidgetsOfClass` "/Game/UI/Blueprints/SettingsMenu/SettingsUI.SettingsUI_C"))
  (bind _output (`|GetArrayItem` _foundwidgets))
  (`/Engine/EditorBlueprintResources/StandardMacros.IsValid` _output
    (:`Is Valid`
      (`Widget.RemoveFromParent` _output))))

(event `InputAction|PauseMenu` :paused true
  (params (Key :type "Key Structure"))
  ;[1 1 1] PauseMenu
  (:`Pressed`
    (set `self.GamepadInput` (`KismetInputLibrary.Key_IsGamepadKey` Key))
    (if (`self.bMenuOpen`)
      (`self.CloseMenu`)
      (else
        (`self.OpenMenu`)))))

(event `InputAction|ResetCourse`
  (params (Key :type "Key Structure"))
  ;[1 1 1] ResetCourse
  (:`Pressed`
    (`self.SetLevel`)))

(event `Key|One`
  (params (Key :type "Key Structure"))
  (:`Pressed`
    (`GameplayStatics.OpenLevelBySoftObjectPtr` "/Game/Maps/TestLevel_1.TestLevel_1")))

(event `Key|Two`
  (params (Key :type "Key Structure"))
  (:`Pressed`
    (`GameplayStatics.SetGlobalTimeDilation` 1.0)))

(event `Key|Three`
  (params (Key :type "Key Structure"))
  (:`Pressed`
    (`GameplayStatics.SetGlobalTimeDilation` 0.25)))

(fn `UserConstructionScript`)